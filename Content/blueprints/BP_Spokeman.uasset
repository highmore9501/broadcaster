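; BP_Spokeman is an NPC character with a name tag that wanders and stops to face nearby players.
; An idle/run/walk/talk state drives movement, looping AI moves through target points or random navigable locations.
; Each tick checks cached BP_Character_Pei distances, entering Talk up close and restoring the previous state after a delay.
; A separate SaySth event plays the current sound, and name setup retries by timer until the widget exists.
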(event Custom|SaySth
  (bind _audio (Variables|Default|GetAudio))
  (Audio|Components|Audio|SetSound _audio (Variables|Sound|Getcurrent_sound))
  (Audio|Components|Audio|Play _audio 0.0))

(event Custom|NPC_movement
  (bind _charactermovement (Variables|Character|GetCharacterMovement))
  (switch Utilities|FlowControl|Switch|SwitchonEnum_NPC_State (Variables|Nav|Getnpc_state)
    (:NewEnumerator0
      (Variables|Default|SetisMoving false :!label _label))
    (:NewEnumerator1
      (Variables|/Script/Engine.CharacterMovementComponent|SetMaxWalkSpeed _charactermovement 6e+02)
      (if (Variables|Nav|GetrandomNav) :!label _label_2
        (CallFunction|RandomMove)
        (else
          (CallFunction|MovebyTargetPoints)))
      (Variables|Default|SetisMoving true))
    (:NewEnumerator2
      (Variables|/Script/Engine.CharacterMovementComponent|SetMaxWalkSpeed _charactermovement 3e+02)
      (goto _label_2))
    (:NewEnumerator3
      (goto _label))))

(event Custom|MoveByTargetPoints
  (AI|AIMoveTo self "0, 0, 0" (Utilities|Array|Get(acopy) (Variables|Nav|Gettarget_points) (Variables|Nav|Gettarget_index)) 5.0 false :!label _label
    (:OnSuccess
      (if (== (+ (Variables|Nav|Gettarget_index) 1) (Utilities|Array|Length (Variables|Nav|Gettarget_points)))
        (Development|PrintString "target array finished!")
        (Variables|Nav|Settarget_index 0)
        (else
          (Development|PrintString "next target!")
          (Variables|Nav|Settarget_index (+ (Variables|Nav|Gettarget_index) 1))))
      (if (Variables|Default|GetisMoving)
        (goto _label)
        (else
          (Development|PrintString "STOP MOVE"))))))

(event Custom|RandomMove
  (bind _self self)
  (bind _randomlocation (Class|NavigationSystemV1|GetRandomLocationinNavigableRadius (Pawn|GetNavAgentLocation _self) 1e+03 0 0 :!label _label))
  (AI|AIMoveTo _self _randomlocation 0 5.0 false
    (:OnSuccess
      (if (Variables|Default|GetisMoving)
        (goto _label)
        (else
          (Development|PrintString "STOP MOVE"))))))

(event Custom|updatePlayers
  (bind _outactors (Actor|GetAllActorsOfClass "/Game/blueprints/Pei/BP_Character_Pei.BP_Character_Pei_C"))
  (bind _output_get (Variables|Nav|Setplayers _outactors))
  (for _array_element _output_get
    _))

(event Custom|CheckForPlayerTalk
  (bind _self self)
  (for _array_element (Variables|Nav|Getplayers)
    (if (and (Utilities|Enum|NotEqual(Enum) (Variables|Nav|Getnpc_state) "NewEnumerator3") (<= (Transformation|GetDistanceTo _array_element self) 1e+02))
      (Variables|Nav|Setpre_npc_state (Variables|Nav|Getnpc_state))
      (Variables|Nav|Setnpc_state "NewEnumerator3")
      (Variables|Default|Setnpc_state_changed true)
      (Components|Movement|StopMovementImmediately (Variables|Character|GetCharacterMovement))
      (Transformation|SetActorRotation _self (Math|Rotator|MakeRotator (.roll (Math|Rotator|FindLookatRotation (Transformation|GetActorLocation _self) (Transformation|GetActorLocation _array_element))) 0.0 (.yaw (Math|Rotator|FindLookatRotation (Transformation|GetActorLocation _self) (Transformation|GetActorLocation _array_element)))))
      (elif (and (!= (<= (Transformation|GetDistanceTo _array_element self) 1e+02) true) (Utilities|Enum|Equal(Enum) (Variables|Nav|Getnpc_state) "NewEnumerator3"))
        (Utilities|FlowControl|Delay 3.0)
        (Variables|Nav|Setnpc_state (Variables|Nav|Getpre_npc_state))
        (Variables|Default|Setnpc_state_changed true)))))

(event EventBeginPlay
  (CallFunction|SetupName)
  (CallFunction|NPCMovement)
  (Variables|Default|Setnpc_state_changed false)
  (CallFunction|UpdatePlayers)
  (Variables|Nav|Setpre_npc_state "NewEnumerator2"))

(event EventTick
  (params (DeltaSeconds :type Float%20%28single-precision%29))
  (if (Variables|Default|Getnpc_state_changed)
    (CallFunction|NPCMovement)
    (Variables|Default|Setnpc_state_changed false))
  (CallFunction|CheckforPlayerTalk))

(fn ConstructionScript)

(fn SetupName
  (bind _nametagwidget (Variables|Default|GetnameTagWidget))
  (bind _returnvalue (UserInterface|GetWidget _nametagwidget))
  (if (Utilities|IsValid _returnvalue)
    (bind _aswb_name_tag (Utilities|Casting|CastToWB_NameTag _returnvalue))
    (Variables|/Script/UMG.EditableTextBox|SetText (Variables|/Game/blueprints/widget/WB_NameTag.WB_NameTag_C|Getplayer_name _aswb_name_tag) (Variables|Default|GetspokemanName))
    (else
      (Utilities|Time|SetTimerbyFunctionName 0 "setupName" 0.1))))