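; Player character Blueprint for Pei, with Enhanced Input movement, jump, Shift sprint and a minimap widget created on begin play.
; Camera look applies only while a mouse button is held, and the cursor hides during the hold.
; Bracket keys zoom the spring arm within limits.
; SaveVoiceFiles passes voice IDs to the NpcTalk component and runs its voice task, while F prints the stored voice file entries for debugging.
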(event Custom|SaveVoiceFiles
  (params (Voice%20Ids :type Array%20of%20Strings))
  (Class|NpcTalkComponent|SaveVoiceFile (Variables|Default|GetNpcTalk) Voice%20Ids)
  (Class|NpcTalkComponent|ExecuteVoiceTask (Variables|Default|GetNpcTalk)))

(event Custom|SetSpringArm
  (params (SpringArmLength :type Float%20%28double-precision%29))
  (bind _output_get (Variables|Default|SetSpringArmLength SpringArmLength))
  (Variables|/Script/Engine.SpringArmComponent|SetTargetArmLength (Variables|Default|GetSpringArm) _output_get))

(event Input|EnhancedActionEvents|EnhancedInputActionIA_jump
  (params (ActionValue :type Boolean) (ElapsedSeconds :type Float%20%28double-precision%29) (TriggeredSeconds :type Float%20%28double-precision%29) (InputAction :type Input%20Action%20Object%20Reference :default "/Game/blueprints/IA_jump.IA_jump"))
  (:Started
    (Character|Jump))
  (:Completed
    (Character|StopJumping)))

(event Input|EnhancedActionEvents|EnhancedInputActionIA_look
  (params (ActionValue :type Vector%202D%20Structure) (ElapsedSeconds :type Float%20%28double-precision%29) (TriggeredSeconds :type Float%20%28double-precision%29) (InputAction :type Input%20Action%20Object%20Reference :default "/Game/blueprints/IA_look.IA_look"))
  (if (or (Variables|Default|GetRightMouseHold) (Variables|Default|GetLeftMouseHold))
    (Pawn|Input|AddControllerYawInput (.x ActionValue))
    (Pawn|Input|AddControllerPitchInput (.y ActionValue))))

(event Input|EnhancedActionEvents|EnhancedInputActionIA_move
  (params (ActionValue :type Vector%202D%20Structure) (ElapsedSeconds :type Float%20%28double-precision%29) (TriggeredSeconds :type Float%20%28double-precision%29) (InputAction :type Input%20Action%20Object%20Reference :default "/Game/blueprints/IA_move.IA_move"))
  (bind _returnvalue (Pawn|GetControlRotation :!class /Script/Engine.Pawn))
  (Pawn|Input|AddMovementInput (Math|Vector|GetRightVector (Pawn|GetControlRotation :!class /Script/Engine.Pawn)) (.x ActionValue) false)
  (Pawn|Input|AddMovementInput (Math|Vector|GetForwardVector (Math|Rotator|MakeRotator (.roll _returnvalue) 0.0 (.yaw _returnvalue))) (.y ActionValue) false))

(event EventBeginPlay
  (bind _returnvalue (Pawn|GetLocalViewingPlayerController))
  (Utilities|IsValid _returnvalue
    (:Is%20Valid
      (Input|AddMappingContext (PlayerController|LocalPlayerSubsystems|GetEnhancedInputLocalPlayerSubsystem _returnvalue) "/Game/blueprints/IMC_Pei.IMC_Pei" 0 "(bIgnoreAllPressedKeysUntilRelease=True,bForceImmediately=False,bNotifyUserSettings=False)")
      (Input|SetInputModeGameandUI _returnvalue 0 "DoNotLock" true false)
      (bind _returnvalue_2 (UserInterface|CreateWidget "/Game/blueprints/widget/WB_Minimap.WB_Minimap_C" (Pawn|GetLocalViewingPlayerController)))
      (UserInterface|Viewport|AddtoViewport _returnvalue_2 0))))

(event Input|MouseEvents|LeftMouseButton
  (params (Key :type Key%20Structure :default "None"))
  (:Pressed
    (Variables|Default|SetLeftMouseHold true)
    (bind _assuper_player_controller (Utilities|Casting|CastToSuper_PlayerController (Pawn|GetLocalViewingPlayerController) :!label _label))
    (Variables|/Script/Engine.PlayerController|SetbShowMouseCursor _assuper_player_controller (and (!= (Variables|Default|GetRightMouseHold) true) (!= (Variables|Default|GetLeftMouseHold) true))))
  (:Released
    (Variables|Default|SetLeftMouseHold false)
    (goto _label)))

(event Input|MouseEvents|RightMouseButton
  (params (Key :type Key%20Structure :default "None"))
  (:Pressed
    (Variables|Default|SetRightMouseHold true)
    (bind _assuper_player_controller (Utilities|Casting|CastToSuper_PlayerController (Pawn|GetLocalViewingPlayerController) :!label _label))
    (Variables|/Script/Engine.PlayerController|SetbShowMouseCursor _assuper_player_controller (and (!= (Variables|Default|GetRightMouseHold) true) (!= (Variables|Default|GetLeftMouseHold) true))))
  (:Released
    (Variables|Default|SetRightMouseHold false)
    (goto _label)))

(event Input|KeyboardEvents|LeftShift
  (params (Key :type Key%20Structure :default "None"))
  (bind _charactermovement (Variables|Character|GetCharacterMovement))
  (:Pressed
    (Variables|Default|SetAccelerate true)
    (Variables|/Script/Engine.CharacterMovementComponent|SetMaxWalkSpeed _charactermovement 1.2e+03))
  (:Released
    (Variables|Default|SetAccelerate false)
    (Variables|/Script/Engine.CharacterMovementComponent|SetMaxWalkSpeed _charactermovement 6e+02)))

(event Input|KeyboardEvents|LeftBracket
  (params (Key :type Key%20Structure :default "None"))
  (bind _springarm (Variables|Default|GetSpringArm))
  (bind _targetarmlength (Variables|/Script/Engine.SpringArmComponent|GetTargetArmLength _springarm))
  (bind _returnvalue (- _targetarmlength 1e+01))
  (:Pressed
    (if (>= _returnvalue 3e+01)
      (CallFunction|SetSpringArm _returnvalue))))

(event Input|KeyboardEvents|RightBracket
  (params (Key :type Key%20Structure :default "None"))
  (bind _springarm (Variables|Default|GetSpringArm))
  (bind _targetarmlength (Variables|/Script/Engine.SpringArmComponent|GetTargetArmLength _springarm))
  (bind _returnvalue (+ _targetarmlength 1e+01))
  (:Pressed
    (if (< _returnvalue 6e+02)
      (CallFunction|SetSpringArm _returnvalue))))

(event Input|KeyboardEvents|F
  (params (Key :type Key%20Structure :default "None"))
  (:Pressed
    (for _array_element (Variables|/Script/broadcaster.NpcTalkComponent|GetVoiceFilesArray (Variables|Default|GetNpcTalk))
      (Development|PrintString (Utilities|String|Append (.VoiceId (Utilities|Struct|BreakVoiceFiles _array_element)) "|" (Utilities|GetDisplayName (.VoiceFile (Utilities|Struct|BreakVoiceFiles _array_element))) "|" (Utilities|GetDisplayName (.VoiceFileJson (Utilities|Struct|BreakVoiceFiles _array_element))))))))

(fn ConstructionScript)