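; Player controller for AI-voiced chat with selectable BP_Spokeman NPCs, creating the local chat UI and tracking the selected NPC.
; Committed chat updates the UI and, with an NPC targeted, POSTs the text through VaRest.
; The response is routed to the name-matched controller, which downloads and plays the WAV via a streaming sound wave, saves lip-sync JSON to file and shows the AI reply.
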(event Custom|updateCurrentSpokeMan
  (params (isSelected :type Boolean) (SpokeMan :type BP%20Spokeman%20Object%20Reference))
  (if isSelected
    (Variables|Default|SetCurrentTarget SpokeMan)
    (elif (== (Variables|Default|GetCurrentTarget) SpokeMan)
      (Variables|Default|SetCurrentTarget 0))))

(event Custom|OC_update_chat
  (params (message :type Text) (player_name :type Text))
  (bind _user_interface (Variables|Default|GetUser%20Interface)
    (:then
      (Default|UpdateChats _user_interface message player_name))
    (:else)))

(event Custom|GetVoiceFiles
  (params (Request%20Data :type String) (NPC%20Name :type Text))
  (bind _returnvalue (|VaRestSubsystem))
  (bind _host (Variables|Default|Gethost))
  (bind _static (Variables|Default|Getstatic))
  (bind _returnvalue_2 (Utilities|String|Append _host _static))
  (bind (_outjsonobject _returnvalue_3) (Class|JsonBlueprintFunctionLibrary|FromString Request%20Data))
  (if _returnvalue_3
    (Utilities|FlowControl|Sequence
      (:then_0
        (bind _outvalue (|GetJsonField _outjsonobject "wav_url"))
        ;[1 1 1] 获得并播放语音
        (Class|VaRestSubsystem|CallURL _returnvalue (Utilities|String|Append _returnvalue_2 _outvalue) "GET" "binary" 0 (delegate Custom|processAudio)))
      (:then_1
        (bind _outvalue_2 (|GetJsonField _outjsonobject "lip_sync_data_url"))
        ;[1 1 1] 处理嘴唇动画
        (Class|VaRestSubsystem|CallURL _returnvalue (Utilities|String|Append _returnvalue_2 _outvalue_2) "GET" "json" 0 (delegate Custom|ProcessText)))
      (:then_2
        (bind _outvalue_3 (|GetJsonField _outjsonobject "ai_reply"))
        (CallFunction|OCUpdateChat _outvalue_3 NPC%20Name)))))

(event Custom|ProcessText
  (params (Request :type Va%20Rest%20Request%20JSON%20Object%20Reference))
  ;[1 1 1] 处理嘴唇动画
  (bind _returnvalue (Class|VaRestRequestJSON|GetResponseContentasString Request true))
  (bind _returnvalue_2 (Class|MyPlayerController|SaveTextFile _returnvalue (stale Custom|GetVoiceFiles _outvalue_2)))
  (Development|PrintString _returnvalue_2))

(event Custom|processAudio
  (params (Request :type Va%20Rest%20Request%20JSON%20Object%20Reference))
  (bind _steaming_sound_wave (Variables|Default|GetSteaming%20Sound%20Wave))
  ;[1 1 1] 获得并播放语音
  (Class|StreamingSoundWave|AppendAudioDatafromEncoded _steaming_sound_wave (Class|VaRestRequestJSON|GetResponseContent Request) "Wav")
  (EventDispatchers|BindEventtoOnAudioPlaybackFinished _steaming_sound_wave (delegate Custom|releaseBuffer))
  (Audio|PlaySound2D _steaming_sound_wave 2.0 1.0 0.0 0 0))

(event Custom|releaseBuffer
  ;[1 1 1] 获得并播放语音
  (bind _returnvalue (Class|StreamingSoundWave|CreateStreamingSoundWave))
  (Variables|Default|SetSteaming%20Sound%20Wave _returnvalue))

(event Custom|dispathMessages
  (params (Request :type Va%20Rest%20Request%20JSON%20Object%20Reference))
  ;[1 1 1] 请求并处理返回的response
  (bind _returnvalue (Class|VaRestRequestJSON|GetResponseContentasString Request true))
  (Utilities|String|LogString _returnvalue)
  (for _array_element (Variables|/Script/Engine.GameStateBase|GetPlayerArray (Game|GetGameState))
    (bind _assuper_player_controller (Utilities|Casting|CastToSuper_PlayerController (Game|GetPlayerController _array_element)))
    (if (Utilities|Enum|Equal(Enum) (Utilities|GetDisplayName _assuper_player_controller) (Utilities|String|ToString(Text) (stale Custom|SR_commit_chat player_name)))
      (CallFunction|GetVoiceFiles _assuper_player_controller _returnvalue (Variables|/Game/blueprints/BP_Spokeman.BP_Spokeman_C|GetspokemanName (stale Custom|SR_commit_chat _asbp_spokeman))))))

(event Custom|requestFailed
  (params (Request :type Va%20Rest%20Request%20JSON%20Object%20Reference))
  ;[1 1 1] 请求并处理返回的response
  (bind _returnvalue (Class|VaRestRequestJSON|GetResponseContentasString Request true))
  (Development|PrintString _returnvalue))

(event Custom|SR_commit_chat
  (params (chat_message :type Text) (player_name :type Text))
  (CallFunction|OCUpdateChat chat_message player_name)
  (bind _currenttarget (Variables|Default|GetCurrentTarget)
    (:then
      (bind _asbp_spokeman (Utilities|Casting|CastToBP_Spokeman _currenttarget))
      (bind _request (CallFunction|ConstructAIVoiceRequest chat_message (Variables|/Game/blueprints/BP_Spokeman.BP_Spokeman_C|Getnpc_background _asbp_spokeman)))
      ;[1 1 1] 请求并处理返回的response
      (EventDispatchers|BindEventtoOnRequestComplete _request (delegate Custom|dispathMessages))
      (EventDispatchers|BindEventtoOnRequestFail _request (delegate Custom|requestFailed))
      (Class|VaRestRequestJSON|ExecuteProcessRequest _request))
    (:else)))

(event EventBeginPlay
  (if (Pawn|IsLocalPlayerController)
    (bind _returnvalue (UserInterface|CreateWidget "/Game/blueprints/widget/WB_UserInterface.WB_UserInterface_C" self))
    (bind _output_get (Variables|Default|SetUser%20Interface _returnvalue))
    (UserInterface|Viewport|AddtoViewport _output_get 0)
    (bind _returnvalue_2 (Class|StreamingSoundWave|CreateStreamingSoundWave))
    (Variables|Default|SetSteaming%20Sound%20Wave _returnvalue_2)
    (bind _outactors (Actor|GetAllActorsOfClass "/Game/blueprints/BP_Spokeman.BP_Spokeman_C"))
    (for _array_element _outactors
      (EventDispatchers|BindEventtoSelected _array_element (delegate Custom|updateCurrentSpokeMan)))))

(event Input|KeyboardEvents|Enter
  (params (Key :type Key%20Structure :default "None"))
  (:Pressed
    (bind _user_interface (Variables|Default|GetUser%20Interface)
      (:then
        (Widget|SetKeyboardFocus (Variables|/Game/blueprints/widget/WB_UserInterface.WB_UserInterface_C|Getuser_input _user_interface)))
      (:else))))

(fn ConstructionScript)

(fn ConstructAIVoiceRequest
  (params (Chat%20Message :type Text) (NPCPrompt :type Text))
  (bind _texts (Variables|Default|GetTexts))
  (if (Utilities|Enum|Equal(Enum) (Utilities|String|ToString(Text) NPCPrompt) (PlayerState|GetPlayerName (Variables|Default|GetPlayerState self)))
    (Utilities|Array|Clear _texts)
    (Utilities|Array|Add _texts (Utilities|String|ToString(Text) Chat%20Message))
    (bind (_outjsonstring _returnvalue) (|StructtoJsonString (Utilities|Struct|MakeVoiceRequestBody (Variables|Default|GetTexts) (Utilities|String|ToString(Integer) (Math|Random|RandomInteger 50000)))))
    (if _returnvalue
      (bind _returnvalue_2 (Class|VaRestSubsystem|ConstructVaRestRequestExt (|VaRestSubsystem) "POST" "x_www_form_urlencoded_body"))
      (Class|VaRestRequestJSON|SetURL _returnvalue_2 (Utilities|String|Append (Variables|Default|Gethost) (Variables|Default|Getendpoint)))
      (Class|VaRestRequestJSON|SetHeader _returnvalue_2 "Content-Type" "application/json")
      (Development|PrintString _outjsonstring)
      (Class|VaRestRequestJSON|SetStringRequestContent _returnvalue_2 _outjsonstring)
      (return _returnvalue_2))))